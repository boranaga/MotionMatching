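; BP_Parcel is a parcel actor that fades out and destroys itself after resting in a BP_Goal.
; Tick polls the Cube's overlaps, incrementing GoalingTime per frame (not by delta time) and resetting it outside the goal.
; Past the threshold, Clear lowers material opacity each frame via CreateDynamicMaterialInstance until destruction.
; Leaving the goal keeps the faded opacity, destroying the parcel if already nearly transparent.
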(event EventBeginPlay
  (Variables|Default|SetOpacityScalar 1.0))

(event Collision|EventActorBeginOverlap
  (params (OtherActor :type Actor%20Object%20Reference)))

(event EventTick
  (params (DeltaSeconds :type Float%20%28single-precision%29))
  (if (> (Utilities|Array|Length (Collision|GetOverlappingActors (Variables|Default|GetCube) "/Game/GameObject/BP_Goal.BP_Goal_C" :!class /Script/Engine.PrimitiveComponent)) 0)
    (Variables|Default|SetGoalingTime (+ (Variables|Default|GetGoalingTime) 0.01))
    (if (> (Variables|Default|GetGoalingTime) 3.0)
      (CallFunction|Clear))
    (elif (< (Variables|Default|GetOpacityScalar) 0.1)
      (Actor|DestroyActor)
      (else
        (Variables|Default|SetGoalingTime 0.0)))))

(fn ConstructionScript)

(fn Clear
  (bind _returnvalue (Rendering|Material|CreateDynamicMaterialInstance (Variables|Default|GetCube) 0 "/Game/GameObject/m_ParcelMat_Inst.m_ParcelMat_Inst" "None" :!class /Script/Engine.PrimitiveComponent))
  (Rendering|Material|SetScalarParameterValue _returnvalue "Opacity" (- (Variables|Default|GetOpacityScalar) 0.005) :!class /Script/Engine.MaterialInstanceDynamic)
  (bind _output_get (Variables|Default|SetOpacityScalar (- (Variables|Default|GetOpacityScalar) 0.005)))
  (if (< _output_get 0.05)
    (Actor|DestroyActor)))